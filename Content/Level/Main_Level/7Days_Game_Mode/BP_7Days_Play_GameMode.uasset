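; Game mode for the 7 Days play mode that tracks whether zombie spawning is on, based on the day/night state.
; Every tick it reads IsDay from the C_STSInstance game instance, clearing the ZombieSpawn flag by day and setting it at night.
; It only maintains the flag and contains no spawning logic; BeginPlay also enables input for the first player controller.
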(event EventBeginPlay
  (Input|EnableInput (Game|GetPlayerController 0)))

(event EventTick
  (params (DeltaSeconds :type Float%20%28single-precision%29))
  (bind _asc_stsinstance (Utilities|Casting|CastToC_STSInstance (Game|GetGameInstance)))
  (if (Variables|/Script/Sevendays_to_survive.C_STSInstance|GetIsDay _asc_stsinstance)
    (Variables|Default|SetZombieSpawn false)
    (elif (not (Variables|Default|GetZombieSpawn))
      (Variables|Default|SetZombieSpawn true))))

(fn ConstructionScript)