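; BP_EnddingPoint is a destination actor in the CityPark level that tracks whether the player has arrived at the end point.
; On BeginPlay with authority, it writes its location into the first player's BP_NickPlayer NaviVec.
; Its Sphere's begin and end overlaps call SetPlayerArrive, which accepts only player pawn 0 as a C_GlobalPlayer.
; That function sets PlayerArrive on the C_STSInstance game instance unless GameEnd is already set.
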(event OnComponentBeginOverlap(Sphere)
  (params (OverlappedComponent :type Primitive%20Component%20Object%20Reference) (OtherActor :type Actor%20Object%20Reference) (OtherComp :type Primitive%20Component%20Object%20Reference) (OtherBodyIndex :type Integer) (bFromSweep :type Boolean) (SweepResult :type Hit%20Result%20Structure%20%28by%20ref%29))
  (CallFunction|SetPlayerArrive OtherActor true))

(event OnComponentEndOverlap(Sphere)
  (params (OverlappedComponent :type Primitive%20Component%20Object%20Reference) (OtherActor :type Actor%20Object%20Reference) (OtherComp :type Primitive%20Component%20Object%20Reference) (OtherBodyIndex :type Integer))
  (CallFunction|SetPlayerArrive OtherActor false))

(event EventBeginPlay
  (if (Ability|HasAuthority)
    (bind _asbp_nick_player (Utilities|Casting|CastToBP_NickPlayer (Game|Player|GetPlayerPawn 0)))
    (Variables|/Game/Level/TestLevel/CharTest/Player/MainPlayer/BP_NickPlayer.BP_NickPlayer_C|SetNaviVec _asbp_nick_player (Transformation|GetActorLocation))))

(event EventTick
  (params (DeltaSeconds :type Float%20%28single-precision%29)))

(fn ConstructionScript)

(fn SetPlayerArrive
  (params (Other%20Actor :type Actor%20Object%20Reference) (Is%20Arrived :type Boolean))
  (bind _asc_global_player (Utilities|Casting|CastToC_GlobalPlayer Other%20Actor))
  (if (== (Game|Player|GetPlayerPawn 0) _asc_global_player)
    (bind _asc_stsinstance (Utilities|Casting|CastToC_STSInstance (Game|GetGameInstance)))
    (if (not (Variables|/Script/Sevendays_to_survive.C_STSInstance|GetGame_End _asc_stsinstance))
      (bind _asc_stsinstance_2 (Utilities|Casting|CastToC_STSInstance (Game|GetGameInstance)))
      (Variables|/Script/Sevendays_to_survive.C_STSInstance|SetPlayer_arrive _asc_stsinstance_2 Is%20Arrived))))