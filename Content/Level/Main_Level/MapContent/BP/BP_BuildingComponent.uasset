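; BP_BuildingComponent is the input layer for a building system in which the player holds, rotates and places building parts.
; Debug-mode test inputs call HoldBuildingPart with wood foundation, door frame, wall, door or none.
; Holding the rotate input runs a fast looping timer that calls RotatePreview, cleared on release or cancel.
; The place input calls PlaceBuildPart; BeginPlay and Tick are empty.
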(event Custom|Rotate%20Preview%20Delegate
  ;[1 1 1] IA_RotateBuilding
  (Class|CBuildingComponent|RotatePreview))

(event Input|EnhancedActionEvents|EnhancedInputActionIA_Test_HoldWoodDoorFrame
  (params (ActionValue :type Boolean) (ElapsedSeconds :type Float%20%28double-precision%29) (TriggeredSeconds :type Float%20%28double-precision%29) (InputAction :type Input%20Action%20Object%20Reference :default "/Game/Level/Main_Level/MapContent/Input/IA_Test_HoldWoodDoorFrame.IA_Test_HoldWoodDoorFrame"))
  (:Started
    (if (Variables|Default|GetBSDebugMode)
      (Class|CBuildingComponent|HoldBuildingPart "WoodDoorFrame"))))

(event Input|EnhancedActionEvents|EnhancedInputActionIA_PlaceBuilding
  (params (ActionValue :type Boolean) (ElapsedSeconds :type Float%20%28double-precision%29) (TriggeredSeconds :type Float%20%28double-precision%29) (InputAction :type Input%20Action%20Object%20Reference :default "/Game/Level/Main_Level/MapContent/Input/IA_PlaceBuilding.IA_PlaceBuilding"))
  ;[1 1 1] Place BuildPart
  (:Started
    (Class|CBuildingComponent|PlaceBuildPart)))

(event Input|EnhancedActionEvents|EnhancedInputActionIA_RotateBuilding
  (params (ActionValue :type Boolean) (ElapsedSeconds :type Float%20%28double-precision%29) (TriggeredSeconds :type Float%20%28double-precision%29) (InputAction :type Input%20Action%20Object%20Reference :default "/Game/Level/Main_Level/MapContent/Input/IA_RotateBuilding.IA_RotateBuilding"))
  ;[1 1 1] IA_RotateBuilding
  (:Started
    (bind _returnvalue (Utilities|Time|SetTimerbyEvent (delegate Custom|Rotate%20Preview%20Delegate) 0.01 true)) ; 0.01초 마다 Rotate Preview 이벤트를 발생시킨다.
    (Variables|Default|SetBP_RotateTimerHandle _returnvalue))
  (:Canceled
    (Utilities|Time|ClearandInvalidateTimerbyHandle (Variables|Default|GetBP_RotateTimerHandle) :!label _label)
    (Variables|Default|SetBP_RotateTimerHandle ""))
  (:Completed
    (goto _label)))

(event Input|EnhancedActionEvents|EnhancedInputActionIA_Test_HoldNone
  (params (ActionValue :type Boolean) (ElapsedSeconds :type Float%20%28double-precision%29) (TriggeredSeconds :type Float%20%28double-precision%29) (InputAction :type Input%20Action%20Object%20Reference :default "/Game/Level/Main_Level/MapContent/Input/IA_Test_HoldNone.IA_Test_HoldNone"))
  (:Started
    (if (Variables|Default|GetBSDebugMode)
      (Class|CBuildingComponent|HoldBuildingPart "None"))))

(event Input|EnhancedActionEvents|EnhancedInputActionIA_Test_HoldWoodFoundation
  (params (ActionValue :type Boolean) (ElapsedSeconds :type Float%20%28double-precision%29) (TriggeredSeconds :type Float%20%28double-precision%29) (InputAction :type Input%20Action%20Object%20Reference :default "/Game/Level/Main_Level/MapContent/Input/IA_Test_HoldWoodFoundation.IA_Test_HoldWoodFoundation"))
  (:Started
    (if (Variables|Default|GetBSDebugMode)
      (Class|CBuildingComponent|HoldBuildingPart "WoodFoundation"))))

(event Input|EnhancedActionEvents|EnhancedInputActionIA_Test_HoldWoodWall
  (params (ActionValue :type Boolean) (ElapsedSeconds :type Float%20%28double-precision%29) (TriggeredSeconds :type Float%20%28double-precision%29) (InputAction :type Input%20Action%20Object%20Reference :default "/Game/Level/Main_Level/MapContent/Input/IA_Test_HoldWoodWall.IA_Test_HoldWoodWall"))
  (:Started
    (if (Variables|Default|GetBSDebugMode)
      (Class|CBuildingComponent|HoldBuildingPart "WoodWall"))))

(event Input|EnhancedActionEvents|EnhancedInputActionIA_Test_HoldWoodDoor
  (params (ActionValue :type Boolean) (ElapsedSeconds :type Float%20%28double-precision%29) (TriggeredSeconds :type Float%20%28double-precision%29) (InputAction :type Input%20Action%20Object%20Reference :default "/Game/Level/Main_Level/MapContent/Input/IA_Test_HoldWoodDoor.IA_Test_HoldWoodDoor"))
  (:Started
    (if (Variables|Default|GetBSDebugMode)
      (Class|CBuildingComponent|HoldBuildingPart "WoodDoor"))))

(event EventBeginPlay
  ;[1 1 1] BeginPlay
)

(event EventTick
  (params (DeltaSeconds :type Float%20%28single-precision%29))
  ;[1 1 1] Tick
)