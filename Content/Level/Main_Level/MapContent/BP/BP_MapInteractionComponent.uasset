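; BP_MapInteractionComponent detects map items in front of the locally controlled player and lets that player interact with item pouches.
; Each tick it runs two box traces along the camera-oriented HP bar trace segment, one object channel for item sources and one for item pouches.
; Each result goes to its own processing function, defined outside this graph.
; The IA_MapInteract input calls MapInteract on the currently viewed item pouch, if valid.
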(event Input|EnhancedActionEvents|EnhancedInputActionIA_MapInteract
  (params (ActionValue :type Boolean) (ElapsedSeconds :type Float%20%28double-precision%29) (TriggeredSeconds :type Float%20%28double-precision%29) (InputAction :type Input%20Action%20Object%20Reference :default "/Game/Level/Main_Level/MapContent/Input/IA_MapInteract.IA_MapInteract"))
  (:Started
    (if (Utilities|IsValid (Variables|Default|GetViewingItemPouch))
      (Class|CMapInteractable|MapInteract (Variables|Default|GetViewingItemPouch)))))

(event EventBeginPlay)

(event EventTick
  (params (DeltaSeconds :type Float%20%28single-precision%29))
  (if (Class|CMapInteractionComponent|IsOwnerLocallyControlled)
    (bind (_outhit _returnvalue) (Class|KismetSystemLibrary|BoxTraceSingleforObjects (Class|CMapInteractionComponent|GetHpBarTraceStartPoint) (Class|CMapInteractionComponent|GetHpBarTraceEndPoint) (/ (Variables|Default|GetHpBarLineTraceBoxSize) 2) (Class|CMapInteractionComponent|GetCameraRotation) (Utilities|Array|MakeArray "ObjectTypeQuery7") false 0 "None" true "(R=1.000000,G=0.000000,B=0.000000,A=1.000000)" "(R=0.000000,G=1.000000,B=0.000000,A=1.000000)" 0.1))
    (Class|CMapInteractionComponent|ProcessItemSourceTraceResult _outhit _returnvalue)
    (bind (_outhit_2 _returnvalue_2) (Class|KismetSystemLibrary|BoxTraceSingleforObjects (Class|CMapInteractionComponent|GetHpBarTraceStartPoint) (Class|CMapInteractionComponent|GetHpBarTraceEndPoint) (/ (Variables|Default|GetHpBarLineTraceBoxSize) 2) (Class|CMapInteractionComponent|GetCameraRotation) (Utilities|Array|MakeArray "ObjectTypeQuery9") false 0 "None" true "(R=1.000000,G=0.000000,B=0.000000,A=1.000000)" "(R=0.000000,G=1.000000,B=0.000000,A=1.000000)" 0.1))
    (Class|CMapInteractionComponent|ProcessItemPouchTraceResult _outhit_2 _returnvalue_2)))