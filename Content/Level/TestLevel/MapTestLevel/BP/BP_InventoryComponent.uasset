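; Inventory component Blueprint that periodically prints its owner's item count as on-screen debug output.
; On BeginPlay it starts a looping timer only when its owner is the pawn controlled by player controller 0.
; Each timer tick calls Report, which prints a label and the GetItemCount result; the component's Tick event is unused.
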(event Custom|Report
  (Development|PrintString "Item Count:" true true "(R=0.000000,G=0.660000,B=1.000000,A=1.000000)" 5.0)
  (Development|PrintString (Utilities|String|ToString(Integer) (Class|CInventoryComponent|GetItemCount)) true true "(R=0.000000,G=0.660000,B=1.000000,A=1.000000)" 5.0))

(event EventBeginPlay
  (if (== (Pawn|GetControlledPawn (Game|GetPlayerController 0)) (Components|GetOwner))
    (Utilities|Time|SetTimerbyEvent (delegate Custom|Report) 1e+01 true)))

(event EventTick
  (params (DeltaSeconds :type Float%20%28single-precision%29)))