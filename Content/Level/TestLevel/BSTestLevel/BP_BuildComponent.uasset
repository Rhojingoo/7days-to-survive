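; Build-mode component for BP_BSTestCharacter that previews and places buildings loaded from the DT_Building data table.
; Input toggles the mode, rotates the build transform and spawns the selected actor; the mouse wheel changes the selection.
; While active, Tick line-traces on the building's channel to drive a collisionless preview mesh.
; Socket detection functions match the hit component against sockets reported by the hit actor.
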(event Custom|Rotate%20Preview
  ;[1 1 1] IA_RotateBuilding
)

(event Input|EnhancedActionEvents|EnhancedInputActionIA_ToggleBuildMode
  (params (ActionValue :type Boolean) (ElapsedSeconds :type Float%20%28double-precision%29) (TriggeredSeconds :type Float%20%28double-precision%29) (InputAction :type Input%20Action%20Object%20Reference :default "/Game/Level/TestLevel/BSTestLevel/Input/IA_ToggleBuildMode.IA_ToggleBuildMode"))
  ;[1 1 1] IA_ToggleBuildMode
  (:Started
    (Utilities|FlowControl|FlipFlop
      (:A
        (Variables|Default|SetIs%20Build%20Mode true))
      (:B
        (Variables|Default|SetIs%20Build%20Mode false)
        (Variables|Default|SetCan%20Build false)
        (Components|StaticMesh|SetStaticMesh (Variables|Default|GetPreviewSMComponent) 0)
        (Variables|Default|SetIs%20First%20Preview%20Tick false)))))

(event Input|EnhancedActionEvents|EnhancedInputActionIA_PlaceBuilding
  (params (ActionValue :type Boolean) (ElapsedSeconds :type Float%20%28double-precision%29) (TriggeredSeconds :type Float%20%28double-precision%29) (InputAction :type Input%20Action%20Object%20Reference :default "/Game/Level/TestLevel/BSTestLevel/Input/IA_PlaceBuilding.IA_PlaceBuilding"))
  ;[1 1 1] IA_PlaceBuilding
  (:Started
    (if (Variables|Default|GetIs%20Build%20Mode)
      (Game|SpawnActorfromClass (.actor (Utilities|Array|Get(acopy) (Variables|Default|GetBuilding%20Struct%20Array) (Variables|Default|GetBuilding%20Struct%20Index))) (Variables|Default|GetBuildTransform) "AlwaysSpawn" "MultiplyWithRoot" 0 0))))

(event Input|EnhancedActionEvents|EnhancedInputActionIA_RotateBuilding
  (params (ActionValue :type Boolean) (ElapsedSeconds :type Float%20%28double-precision%29) (TriggeredSeconds :type Float%20%28double-precision%29) (InputAction :type Input%20Action%20Object%20Reference :default "/Game/Level/TestLevel/BSTestLevel/Input/IA_RotateBuilding.IA_RotateBuilding"))
  ;[1 1 1] IA_RotateBuilding
  (:Started
    (bind _returnvalue (Utilities|Time|SetTimerbyEvent (delegate Custom|Rotate%20Preview) 0.01 true)) ; 0.01초 마다 Rotate Preview 이벤트를 발생시킨다.
    (Variables|Default|SetRotateTimerHandle _returnvalue)
    (Variables|Default|SetBuildTransform (Math|Transform|MakeTransform (.location (Variables|Default|GetBuildTransform)) (Math|Rotator|CombineRotators (.rotation (Variables|Default|GetBuildTransform)) "0.000000,5.000000,0.000000") (.scale (Variables|Default|GetBuildTransform)))))
  (:Canceled
    (Utilities|Time|ClearandInvalidateTimerbyHandle (Variables|Default|GetRotateTimerHandle) :!label _label)
    (Variables|Default|SetRotateTimerHandle ""))
  (:Completed
    (goto _label)))

(event EventBeginPlay
  ;[1 1 1] BeginPlay
  (bind _asbp_bstest_character (Utilities|Casting|CastToBP_BSTestCharacter (Components|GetOwner)))
  (Variables|Default|SetPlayer%20Character _asbp_bstest_character)
  (Variables|Default|SetCameraComponent (Variables|/Game/Level/TestLevel/BSTestLevel/BP_BSTestCharacter.BP_BSTestCharacter_C|GetCamera _asbp_bstest_character))
  (bind _outrownames (DataTable|GetDataTableRowNames "/Game/Level/TestLevel/BSTestLevel/Data/DT_Building.DT_Building"))
  (for _array_element _outrownames
    (bind _returnvalue (Utilities|GetDataTableRow "/Game/Level/TestLevel/BSTestLevel/Data/DT_Building.DT_Building" _array_element)
      (:then
        (Utilities|Array|Add (Variables|Default|GetBuilding%20Struct%20Array) _returnvalue)
        (Variables|Default|SetGreenMaterial "/Game/Level/TestLevel/BSTestLevel/Material/MAT_PreviewGreen.MAT_PreviewGreen")
        (Variables|Default|SetRedMaterial "/Game/Level/TestLevel/BSTestLevel/Material/MAT_PreviewRed.MAT_PreviewRed")))))

(event EventTick
  (params (DeltaSeconds :type Float%20%28single-precision%29))
  ;[1 1 1] Tick
  (if (Variables|Default|GetIs%20Build%20Mode)
    (CallFunction|PreviewTick)))

(event Input|MouseEvents|MouseWheelDown
  (params (Key :type Key%20Structure :default "None"))
  ;[1 1 1] Building Struct Change
  (:Pressed
    (Variables|Default|SetBuilding%20Struct%20Index (Math|Integer|Clamp(Integer) (+ (Variables|Default|GetBuilding%20Struct%20Index) 1) 0 (- (Utilities|Array|Length (Variables|Default|GetBuilding%20Struct%20Array)) 1)))
    (Components|StaticMesh|SetStaticMesh (Variables|Default|GetPreviewSMComponent) 0)
    (Variables|Default|SetIs%20First%20Preview%20Tick true)))

(event Input|MouseEvents|MouseWheelUp
  (params (Key :type Key%20Structure :default "None"))
  ;[1 1 1] Building Struct Change
  (:Pressed
    (Variables|Default|SetBuilding%20Struct%20Index (Math|Integer|Clamp(Integer) (- (Variables|Default|GetBuilding%20Struct%20Index) 1) 0 (- (Utilities|Array|Length (Variables|Default|GetBuilding%20Struct%20Array)) 1)))
    (Components|StaticMesh|SetStaticMesh (Variables|Default|GetPreviewSMComponent) 0)
    (Variables|Default|SetIs%20First%20Preview%20Tick true)))

(fn PreviewTick
  (bind _returnvalue (Class|CBuildComponent|GetLineTraceStartPoint))
  (bind _returnvalue_2 (Class|CBuildComponent|GetLineTraceEndPoint))
  (bind (_outhit _returnvalue_3) (Collision|LineTraceByChannel _returnvalue _returnvalue_2 (.layertracechannel (Utilities|Array|Get(acopy) (Variables|Default|GetBuilding%20Struct%20Array) (Variables|Default|GetBuilding%20Struct%20Index))) false 0 "None"))
  (Variables|Default|SetIsLineTraceHit _returnvalue_3)
  (Utilities|FlowControl|Sequence
    (:then_0
      (if (Variables|Default|GetIs%20First%20Preview%20Tick)
        (Variables|Default|SetIs%20First%20Preview%20Tick false)
        (bind _returnvalue_4 (Game|AddComponentbyClass (Variables|Default|GetPlayer%20Character) "/Script/Engine.StaticMeshComponent" false (Variables|Default|GetBuildTransform)))
        (bind _output_get (Variables|Default|SetPreviewSMComponent _returnvalue_4))
        (Components|StaticMesh|SetStaticMesh _output_get (.staticmesh (Utilities|Array|Get(acopy) (Variables|Default|GetBuilding%20Struct%20Array) (Variables|Default|GetBuilding%20Struct%20Index))))
        (Collision|SetCollisionEnabled _output_get "NoCollision")))
    (:then_1
      (Class|CBuildComponent|SetPreviewTransform (.ImpactPoint (Collision|BreakHitResult _outhit)) (.HitActor (Collision|BreakHitResult _outhit)) (.HitComponent (Collision|BreakHitResult _outhit)) (.TraceEnd (Collision|BreakHitResult _outhit))))))

(fn DetectBuildSockets
  (Variables|Default|SetSocketTransform (Transformation|GetWorldTransform (Variables|Default|GetHitComponent)))
  (bind _newparam (Class|BPIBuildingPart|GetSockets(Message) (Variables|Default|GetHitActor)))
  (bind _array_element (Utilities|Array|ForEachLoopwithBreak _newparam :!label _label)
    (:LoopBody
      (if (== (Variables|Default|GetHitComponent) _array_element)
        (Variables|Default|SetFoundSocket true)
        (goto _label Break)))
    (:Completed
      (return))))

(fn EventDetectSockets
  (Variables|Default|SetSocketTransform (Transformation|GetWorldTransform (Variables|Default|GetHitComponent)))
  (bind _newparam (Class|BPIBuildingPart|GetSockets(Message) (Variables|Default|GetHitActor)))
  (bind _array_element (Utilities|Array|ForEachLoopwithBreak _newparam :!label _label)
    (:LoopBody
      (if (== (Variables|Default|GetHitComponent) _array_element)
        (Variables|Default|SetFoundSocket true)
        (goto _label Break)))
    (:Completed
      (return))))