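; BP_BuildingWall is a wall piece for a building system, located among the test level's building parts.
; A SetMesh event assigns the given mesh to its static mesh component.
; GetSockets returns four box components as the wall's sockets, presumably snap points for attaching other parts.
; The construction script only calls its parent.
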(event Custom|SetMesh
  (params (Mesh :type Static%20Mesh%20Object%20Reference))
  (Components|StaticMesh|SetStaticMesh (Variables|Debug|GetStaticMeshComponent) Mesh))

(fn ConstructionScript
  (|CallParentFunction))

(fn GetSockets
  (return (Utilities|Array|MakeArray (Variables|Default|GetBox1) (Variables|Default|GetBox2) (Variables|Default|GetBox3) (Variables|Default|GetBox))))