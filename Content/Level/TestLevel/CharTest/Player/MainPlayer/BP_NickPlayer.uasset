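; Main player character Blueprint for Nick, layering input, camera and UI setup over native character logic.
; BeginPlay applies the skeletal mesh chosen from BP_STSInstance and, for the first player controller, sets minimap color, map camera and blood overlay.
; Number keys select quick slots, or swap weapon meshes through server calls in develop mode.
; Zoom blends the view to the current weapon with a crosshair, and Tick cancels aiming when hit.
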(event Custom|MultMesh
  (bind _asbp_stsinstance (Utilities|Casting|CastToBP_STSInstance (Game|GetGameInstance)))
  (bind _returnvalue (Class|CSTSInstance|GetPlayerSpawnMesh _asbp_stsinstance))
  (Components|SkeletalMesh|SetSkeletalMeshAsset (Variables|Character|GetMesh) (Utilities|Array|Get(acopy) _returnvalue (Math|Conversions|ToInteger(Byte) (Variables|Default|GetcharacterResultMesh)))))

(event Custom|Server
  (CallFunction|MultMesh))

(event Custom|GetM4Mult
  ;[1 1 1] BP_GetM4Mult
)

(event Custom|M4server
  ;[1 1 1] BP_M4Server
  (CallFunction|GetM4Mult))

(event Custom|LineTrace
  (bind _curweapon (Variables|Default|GetCurWeapon))
  (bind _skeletalmesh (Variables|/Script/Sevendays_to_survive.C_EquipWeapon|GetSkeletalMesh _curweapon))
  (bind _returnvalue (Transformation|GetSocketLocation _skeletalmesh "Muzzle"))
  (bind (_outhit _returnvalue_2) (Collision|LineTraceByChannel _returnvalue (+ _returnvalue (* (Math|Vector|GetForwardVector (Transformation|GetSocketRotation _skeletalmesh "Muzzle")) 1e+04)) "TraceTypeQuery8" false 0 "ForDuration"))
  (if _returnvalue_2
    (Game|SpawnActorfromClass "/Game/Level/TestLevel/CharTest/WeaponSystem_BluePrint/BP_ImPactField.BP_ImPactField_C" (Math|Transform|MakeTransform (.ImpactPoint (Collision|BreakHitResult _outhit)) "0, 0, 0" "1.000000,1.000000,1.000000") "Undefined" "MultiplyWithRoot" 0 0)))

(event Custom|testHit)

(event Input|EnhancedActionEvents|EnhancedInputActionIA_MainMove
  (params (ActionValue :type Vector%202D%20Structure) (ElapsedSeconds :type Float%20%28double-precision%29) (TriggeredSeconds :type Float%20%28double-precision%29) (InputAction :type Input%20Action%20Object%20Reference :default "/Game/Level/TestLevel/CharTest/Player/Input/Action/IA_MainMove.IA_MainMove"))
  (:Started
    (Utilities|FlowControl|DoOnce false
      (:Completed
        (Class|CGlobalPlayer|MeshInit (Variables|Default|GetcharacterResultMesh))
        (CallFunction|Server)))))

(event Input|EnhancedActionEvents|EnhancedInputActionIA_number5Weapon
  (params (ActionValue :type Boolean) (ElapsedSeconds :type Float%20%28double-precision%29) (TriggeredSeconds :type Float%20%28double-precision%29) (InputAction :type Input%20Action%20Object%20Reference :default "/Game/Level/TestLevel/CharTest/Player/Input/Action/IA_number5Weapon.IA_number5Weapon"))
  (:Started
    (if (Variables|Default|GetCharDevelopMode)
      (Class|CGlobalPlayer|ChangeSlotSkeletalServer "RPistol")
      (else
        (Class|CNickMainPlayer|OnQuickSlotSelected 4)))))

(event Input|EnhancedActionEvents|EnhancedInputActionIA_number8Weapon
  (params (ActionValue :type Boolean) (ElapsedSeconds :type Float%20%28double-precision%29) (TriggeredSeconds :type Float%20%28double-precision%29) (InputAction :type Input%20Action%20Object%20Reference :default "/Game/Level/TestLevel/CharTest/Player/Input/Action/IA_number8Weapon.IA_number8Weapon"))
  (:Started
    (if (Variables|Default|GetCharDevelopMode)
      (Class|CGlobalPlayer|ChangeSlotSkeletalServer "RShotgun")
      (else
        (Class|CNickMainPlayer|OnQuickSlotSelected 7)))))

(event Input|EnhancedActionEvents|EnhancedInputActionIA_Zoom
  (params (ActionValue :type Boolean) (ElapsedSeconds :type Float%20%28double-precision%29) (TriggeredSeconds :type Float%20%28double-precision%29) (InputAction :type Input%20Action%20Object%20Reference :default "/Game/Level/TestLevel/CharTest/Player/Input/Action/IA_Zoom.IA_Zoom"))
  (bind _curweapon (Variables|Default|GetCurWeapon))
  (:Started
    (Utilities|IsValid _curweapon
      (:Is%20Valid
        (bind _asbp_main_player_controller (Utilities|Casting|CastToBP_MainPlayerController (Pawn|GetController)))
        (Game|Player|SetViewTargetwithBlend _asbp_main_player_controller (Variables|Default|GetCurWeapon) 0.0 "VTBlend_Linear" 0.0 false)
        (bind _asbp_ui_in_game_hud (Utilities|Casting|CastToBP_UI_InGameHUD (HUD|GetHUD _asbp_main_player_controller)))
        (Widget|SetVisibility (Variables|/Game/Level/TestLevel/UI/WidgetBP/InGame/BP_HealthBar.BP_HealthBar_C|GetCrossHair (Variables|/Game/Level/TestLevel/UI/BP_UI_InGameHUD.BP_UI_InGameHUD_C|GetHPAndAimWidget _asbp_ui_in_game_hud)) "Visible"))))
  (:Completed
    (Utilities|IsValid _curweapon
      (:Is%20Valid
        (bind _asbp_main_player_controller_2 (Utilities|Casting|CastToBP_MainPlayerController (Pawn|GetController)))
        (Game|Player|SetViewTargetwithBlend _asbp_main_player_controller_2 self 0.0 "VTBlend_Linear" 0.0 false)
        (bind _asbp_ui_in_game_hud_2 (Utilities|Casting|CastToBP_UI_InGameHUD (HUD|GetHUD _asbp_main_player_controller_2)))
        (Widget|SetVisibility (Variables|/Game/Level/TestLevel/UI/WidgetBP/InGame/BP_HealthBar.BP_HealthBar_C|GetCrossHair (Variables|/Game/Level/TestLevel/UI/BP_UI_InGameHUD.BP_UI_InGameHUD_C|GetHPAndAimWidget _asbp_ui_in_game_hud_2)) "Hidden")))))

(event Input|EnhancedActionEvents|EnhancedInputActionIA_NoWeapon
  (params (ActionValue :type Boolean) (ElapsedSeconds :type Float%20%28double-precision%29) (TriggeredSeconds :type Float%20%28double-precision%29) (InputAction :type Input%20Action%20Object%20Reference :default "/Game/Level/TestLevel/CharTest/Player/Input/Action/IA_NoWeapon.IA_NoWeapon"))
  (:Started
    (if (Variables|Default|GetCharDevelopMode)
      (Class|CGlobalPlayer|ChangeNoWeaponServer))))

(event Input|EnhancedActionEvents|EnhancedInputActionIA_number3Weapon
  (params (ActionValue :type Boolean) (ElapsedSeconds :type Float%20%28double-precision%29) (TriggeredSeconds :type Float%20%28double-precision%29) (InputAction :type Input%20Action%20Object%20Reference :default "/Game/Level/TestLevel/CharTest/Player/Input/Action/IA_number3Weapon.IA_number3Weapon"))
  (:Started
    (if (Variables|Default|GetCharDevelopMode)
      (Class|CGlobalPlayer|ChangeSlotMeshServer "RAxe" "/Game/Level/TestLevel/CharTest/Axe_OneHanded/Axe_StaticMesh.Axe_StaticMesh")
      (else
        (Class|CNickMainPlayer|OnQuickSlotSelected 2)))))

(event Input|EnhancedActionEvents|EnhancedInputActionIA_numver4Weapon
  (params (ActionValue :type Boolean) (ElapsedSeconds :type Float%20%28double-precision%29) (TriggeredSeconds :type Float%20%28double-precision%29) (InputAction :type Input%20Action%20Object%20Reference :default "/Game/Level/TestLevel/CharTest/Player/Input/Action/IA_numver4Weapon.IA_numver4Weapon"))
  (:Started
    (if (Variables|Default|GetCharDevelopMode)
      (Class|CGlobalPlayer|ChangeSlotSkeletalServer "RPistol2")
      (else
        (Class|CNickMainPlayer|OnQuickSlotSelected 3)))))

(event Input|EnhancedActionEvents|EnhancedInputActionIA_Fire
  (params (ActionValue :type Boolean) (ElapsedSeconds :type Float%20%28double-precision%29) (TriggeredSeconds :type Float%20%28double-precision%29) (InputAction :type Input%20Action%20Object%20Reference :default "/Game/Level/TestLevel/CharTest/Player/Input/Action/IA_Fire.IA_Fire"))
  (:Started
    (Development|PrintString (Utilities|String|ToString(Integer) (Variables|Default|GetLineTracemagazinecapacity)))))

(event Input|EnhancedActionEvents|EnhancedInputActionIA_number6Weapon
  (params (ActionValue :type Boolean) (ElapsedSeconds :type Float%20%28double-precision%29) (TriggeredSeconds :type Float%20%28double-precision%29) (InputAction :type Input%20Action%20Object%20Reference :default "/Game/Level/TestLevel/CharTest/Player/Input/Action/IA_number6Weapon.IA_number6Weapon"))
  (:Started
    (if (Variables|Default|GetCharDevelopMode)
      (Class|CGlobalPlayer|ChangeSlotSkeletalServer "RRifle2")
      (else
        (Class|CNickMainPlayer|OnQuickSlotSelected 5)))))

(event Input|EnhancedActionEvents|EnhancedInputActionIA_number1Weapon
  (params (ActionValue :type Boolean) (ElapsedSeconds :type Float%20%28double-precision%29) (TriggeredSeconds :type Float%20%28double-precision%29) (InputAction :type Input%20Action%20Object%20Reference :default "/Game/Level/TestLevel/CharTest/Player/Input/Action/IA_number1Weapon.IA_number1Weapon"))
  (:Started
    (if (Variables|Default|GetCharDevelopMode)
      (Class|CGlobalPlayer|ChangeSlotMeshServer "RBat" "/Game/Level/TestLevel/CharTest/Bat/bat1.bat1")
      (else
        (Class|CNickMainPlayer|OnQuickSlotSelected)))))

(event Input|EnhancedActionEvents|EnhancedInputActionIA_number2Weapon
  (params (ActionValue :type Boolean) (ElapsedSeconds :type Float%20%28double-precision%29) (TriggeredSeconds :type Float%20%28double-precision%29) (InputAction :type Input%20Action%20Object%20Reference :default "/Game/Level/TestLevel/CharTest/Player/Input/Action/IA_number2Weapon.IA_number2Weapon"))
  (:Started
    (if (Variables|Default|GetCharDevelopMode)
      (Class|CGlobalPlayer|ChangeSlotMeshServer "RSword" "/Game/Level/TestLevel/CharTest/Sword/Sw.Sw")
      (else
        (Class|CNickMainPlayer|OnQuickSlotSelected 1)))))

(event Input|EnhancedActionEvents|EnhancedInputActionIA_number7Weapon
  (params (ActionValue :type Boolean) (ElapsedSeconds :type Float%20%28double-precision%29) (TriggeredSeconds :type Float%20%28double-precision%29) (InputAction :type Input%20Action%20Object%20Reference :default "/Game/Level/TestLevel/CharTest/Player/Input/Action/IA_number7Weapon.IA_number7Weapon"))
  (:Started
    (if (Variables|Default|GetCharDevelopMode)
      (Class|CGlobalPlayer|ChangeSlotSkeletalServer "RRifle")
      (else
        (Class|CNickMainPlayer|OnQuickSlotSelected 6)))))

(event EventBeginPlay
  (Utilities|FlowControl|Sequence
    (:then_0
      (Class|CGlobalPlayer|MeshInit (Variables|Default|GetcharacterResultMesh))
      (CallFunction|MultMesh)
      (CallFunction|Server))
    (:then_1
      ;[1 1 1] 미니맵 내에서 플레이어 컬러 변경
      (if (== (Pawn|GetController) (Game|GetPlayerController 0))
        (Sprite|SetSpriteColor (Variables|Default|GetMinimapIcon) "(R=0.000000,G=1.000000,B=0.019143,A=1.000000)")
        (Utilities|FlowControl|Sequence
          (:then_0
            ;[1 0.5477 0.6076] 몬스터 피격시 모니터 피 애니메이션 -> 위젯으로 옮기기 필요
            (bind _asbp_main_player_controller (Utilities|Casting|CastToBP_MainPlayerController (Pawn|GetController)))
            (Game|Player|SetViewTargetwithBlend _asbp_main_player_controller self 0.0 "VTBlend_Linear" 0.0 false))
          (:then_1
            (Class|CNickMainPlayer|SpawnMapCamera (Math|Transform|MakeTransform (Variables|Default|GetCameraLocation) "0, 0, 0" "1.000000,1.000000,1.000000"))
            (bind _returnvalue (UserInterface|CreateWidget "/Game/Level/TestLevel/UI/WidgetBP/InGame/WB_AttackBloodFX.WB_AttackBloodFX_C"))
            (UserInterface|Viewport|AddtoViewport _returnvalue 0)
            (Variables|Default|SetNaviVec "-53600.000000,2430.000000,0.000000")))))))

(event EventTick
  (params (DeltaSeconds :type Float%20%28single-precision%29))
  (if (Variables|Default|GetIsHitCpp)
    (bind _asbp_main_player_controller (Utilities|Casting|CastToBP_MainPlayerController (Pawn|GetController)))
    (Variables|Default|SetIsAimCpp false)
    (Game|Player|SetViewTargetwithBlend _asbp_main_player_controller self 0.0 "VTBlend_Linear" 0.0 false)
    (bind _asbp_ui_in_game_hud (Utilities|Casting|CastToBP_UI_InGameHUD (HUD|GetHUD _asbp_main_player_controller)))
    (Widget|SetVisibility (Variables|/Game/Level/TestLevel/UI/WidgetBP/InGame/BP_HealthBar.BP_HealthBar_C|GetCrossHair (Variables|/Game/Level/TestLevel/UI/BP_UI_InGameHUD.BP_UI_InGameHUD_C|GetHPAndAimWidget _asbp_ui_in_game_hud)) "Hidden")))

(event Game|Damage|EventAnyDamage
  (params (Damage :type Float%20%28single-precision%29) (DamageType :type Damage%20Type%20Object%20Reference) (InstigatedBy :type Controller%20Object%20Reference) (DamageCauser :type Actor%20Object%20Reference)))

(fn ConstructionScript)

(fn GetWorldRotation
  (return (Transformation|GetWorldRotation (Variables|Default|GetCapsuleComponent))))

(fn GetWorldPostion
  (return (Transformation|GetWorldLocation (Variables|Default|GetCapsuleComponent))))

(fn GetForwardVector
  (return (Math|Vector|GetForwardVector (Variables|Default|GetCapsuleComponent))))