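; BPC_MainAttSystem is the main player's attack component, starting an attack that matches the player's current state.
; The IA_Punchatt input calls the RPCServer event, named as a server RPC.
; That event checks PlayerCurState in sequence, calling AttStart for Sword and AttStart2 for Rifle.
; BeginPlay and Tick are empty.
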(event Custom|RPCServer
  (Utilities|FlowControl|Sequence
    (:then_0
      (if (Utilities|Enum|Equal(Enum) (Variables|/Script/Sevendays_to_survive.C_GlobalPlayer|GetPlayerCurState (Variables|Default|GetPlayer)) "Sword")
        (Class|CMainWeaponAttComponent|AttStart)))
    (:then_1
      (if (Utilities|Enum|Equal(Enum) (Variables|/Script/Sevendays_to_survive.C_GlobalPlayer|GetPlayerCurState (Variables|Default|GetPlayer)) "Rifle")
        (Class|CMainWeaponAttComponent|AttStart2)))))

(event Input|EnhancedActionEvents|EnhancedInputActionIA_Punchatt
  (params (ActionValue :type Boolean) (ElapsedSeconds :type Float%20%28double-precision%29) (TriggeredSeconds :type Float%20%28double-precision%29) (InputAction :type Input%20Action%20Object%20Reference :default "/Game/Level/TestLevel/CharTest/Player/Input/Action/IA_Punchatt.IA_Punchatt"))
  (:Started
    (CallFunction|RPCServer)))

(event EventBeginPlay)

(event EventTick
  (params (DeltaSeconds :type Float%20%28single-precision%29)))