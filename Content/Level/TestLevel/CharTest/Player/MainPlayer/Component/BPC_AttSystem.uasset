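; Melee attack component for BP_NickPlayer that runs a three-hit punch combo of jab, punch and hook.
; Punch input plays the current montage, whose notify unlocks input and advances the combo, while a timer resets the counter.
; StartAttackTrace schedules a debug-drawn sphere trace from the hand matching the combo step, cancellable by stopAttacktrace.
; Left-hand hits damage only BP_ItemSourceHISMA instances by hit index, while right-hand hits use generic ApplyDamage.
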(event Custom|ResetCounter
  (Variables|Default|SetComboCounter 0))

(event Custom|StartAttackTrace
  (bind _returnvalue (Utilities|Time|SetTimerbyEvent (delegate Custom|AttackTrace) 0.01))
  (Variables|Default|SetAttackTimerHandler _returnvalue))

(event Custom|AttackTrace
  (bind _as_bp_nick_player (Variables|Default|GetAs%20BP%20Nick%20Player))
  (bind _as_bp_nick_player_2 (Variables|Default|GetAs%20BP%20Nick%20Player))
  (bind _righthand (Variables|/Game/Level/TestLevel/CharTest/Player/MainPlayer/BP_NickPlayer.BP_NickPlayer_C|GetRightHand _as_bp_nick_player_2))
  (bind _lefthand (Variables|/Game/Level/TestLevel/CharTest/Player/MainPlayer/BP_NickPlayer.BP_NickPlayer_C|GetLeftHand _as_bp_nick_player))
  (bind (_start _end) (CallFunction|GetHandLocation _lefthand))
  (bind (_start_2 _end_2) (CallFunction|GetHandLocation _righthand))
  (switch int (Variables|Default|GetComboCounter)
    (:0
      (bind (_outhit _returnvalue) (Collision|SphereTraceByChannel _start _end 1e+01 "TraceTypeQuery1" false 0 "ForDuration" true "(R=1.000000,G=0.000000,B=0.000000,A=1.000000)" "(R=0.000000,G=1.000000,B=0.000000,A=1.000000)" 7.0 :!label _label))
      (if _returnvalue
        (bind _asbp_item_source_hisma (Utilities|Casting|CastToBP_ItemSourceHISMA (.HitActor (Collision|BreakHitResult _outhit))))
        (Class|CDestructibleHISMA|Damage _asbp_item_source_hisma (.HitItem (Collision|BreakHitResult _outhit)) 10)))
    (:1
      (bind (_outhit_2 _returnvalue_2) (Collision|SphereTraceByChannel _start_2 _end_2 1e+01 "TraceTypeQuery1" false 0 "ForDuration" true "(R=1.000000,G=0.000000,B=0.000000,A=1.000000)" "(R=0.000000,G=1.000000,B=0.000000,A=1.000000)" 7.0))
      (if _returnvalue_2
        (Game|Damage|ApplyDamage (.HitActor (Collision|BreakHitResult _outhit_2)) 1e+01 0 (Variables|Default|GetAs%20BP%20Nick%20Player))))
    (:2
      (goto _label))))

(event Custom|stopAttacktrace
  (Utilities|Time|ClearandInvalidateTimerbyHandle (Variables|Default|GetAttackTimerHandler)))

(event Input|EnhancedActionEvents|EnhancedInputActionIA_Punchatt
  (params (ActionValue :type Boolean) (ElapsedSeconds :type Float%20%28double-precision%29) (TriggeredSeconds :type Float%20%28double-precision%29) (InputAction :type Input%20Action%20Object%20Reference :default "/Game/Level/TestLevel/CharTest/Player/Input/Action/IA_Punchatt.IA_Punchatt"))
  (bind _mesh (Variables|Default|GetMesh))
  (if (not (Variables|Default|GetIsatt))
    (Variables|Default|SetIsatt true)
    (switch int (Variables|Default|GetComboCounter)
      (:0
        (Animation|Montage|PlayMontage _mesh "/Game/Level/TestLevel/CharTest/Player/Woman/Anitest/Attani/Lead_Jab_Montage.Lead_Jab_Montage"
          (:then
            (Utilities|Time|SetTimerbyEvent (delegate Custom|ResetCounter) 1.0 :!label _label))
          (:OnNotifyBegin
            (Variables|Default|SetIsatt false)
            (Variables|Default|SetComboCounter 1))))
      (:1
        (Animation|Montage|PlayMontage _mesh "/Game/Level/TestLevel/CharTest/Player/Woman/Anitest/Attani/Punching_Montage.Punching_Montage"
          (:then
            (goto _label))
          (:OnNotifyBegin
            (Variables|Default|SetIsatt false)
            (Variables|Default|SetComboCounter 2))))
      (:2
        (Animation|Montage|PlayMontage _mesh "/Game/Level/TestLevel/CharTest/Player/Woman/Anitest/Attani/Hook_Montage.Hook_Montage"
          (:then
            (goto _label))
          (:OnNotifyBegin
            (Variables|Default|SetIsatt false)
            (CallFunction|ResetCounter)))))))

(event EventBeginPlay
  (bind _asbp_nick_player (Utilities|Casting|CastToBP_NickPlayer (Components|GetOwner)))
  (bind _output_get (Variables|Default|SetAs%20BP%20Nick%20Player _asbp_nick_player))
  (Variables|Default|SetMesh (Variables|/Script/Engine.Character|GetMesh _output_get)))

(fn GetHandLocation
  (params (Hadn :type Scene%20Component%20Object%20Reference))
  (return (Transformation|GetWorldLocation Hadn) (Math|Transform|TransformLocation (Transformation|GetWorldTransform Hadn) (+ (Variables|/Script/Engine.SceneComponent|GetRelativeLocation Hadn) (Math|Vector|MakeVector 2e+01 0.0 0.0)))))