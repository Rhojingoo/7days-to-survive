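; Player Blueprint that applies a skeletal mesh chosen through the game instance when play begins.
; On BeginPlay it runs the parent logic, then reads the player mesh selection and spawn mesh list from BP_STSInstance.
; The selection is converted to an integer index into that list to set the Mesh component's asset.
; Overlap and Tick events are inactive, and the construction script only calls the parent.
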(event EventBeginPlay
  (|CallParentFunction)
  (bind _asbp_stsinstance (Utilities|Casting|CastToBP_STSInstance (Game|GetGameInstance)))
  (bind _returnvalue (Class|CSTSInstance|GetPlayerMesh _asbp_stsinstance))
  (bind _returnvalue_2 (Class|CSTSInstance|GetPlayerSpawnMesh _asbp_stsinstance))
  (Components|SkeletalMesh|SetSkeletalMeshAsset (Variables|Character|GetMesh) (Utilities|Array|Get(acopy) _returnvalue_2 (Math|Conversions|ToInteger(Byte) _returnvalue))))

(event Collision|EventActorBeginOverlap
  (params (OtherActor :type Actor%20Object%20Reference)))

(event EventTick
  (params (DeltaSeconds :type Float%20%28single-precision%29))
  (|CallParentFunction DeltaSeconds) ; 지금 이 노드는 비활성 상태입니다. \n핀을 끌어서 다른 노드를 연결하면 활성화됩니다.
)

(fn ConstructionScript
  (|CallParentFunction))