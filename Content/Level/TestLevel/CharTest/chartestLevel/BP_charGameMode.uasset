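; Game mode for a character test level that spawns BasicZombie actors at random positions when play begins.
; BeginPlay runs a while loop that spawns one zombie per pass and increments TestInt until it reaches 2.
; Each location takes X and Y from random unit vectors scaled by a random distance, with Z fixed at zero.
; Tick and the construction script are empty.
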(event EventBeginPlay
  (bind _returnvalue (Math|Random|RandomUnitVector))
  (bind _returnvalue_2 (Math|Random|RandomFloat))
  (bind _returnvalue_3 (- _returnvalue_2 -0.5))
  (bind _returnvalue_4 (* _returnvalue_3 2e+03))
  (bind _returnvalue_5 (* _returnvalue _returnvalue_4))
  (bind (_x _y) (Math|Vector|BreakVector _returnvalue_5))
  (while (< (Variables|Default|GetTestInt) 2)
    (Game|SpawnActorfromClass "/Game/MonsterFile/BasicZombie.BasicZombie_C" (Math|Transform|MakeTransform (Math|Vector|MakeVector _x _y 0.0)) "Undefined" "MultiplyWithRoot" 0 0)
    (Variables|Default|SetTestInt (+ (Variables|Default|GetTestInt) 1))))

(event EventTick
  (params (DeltaSeconds :type Float%20%28single-precision%29)))

(fn ConstructionScript)