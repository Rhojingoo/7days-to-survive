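; Player build-mode component for BP_BSTestCharacter that previews and places wooden building foundations.
; While toggled on, a camera line trace each Tick positions a green, collisionless preview mesh, added once per session through a resettable DoOnce.
; Placing spawns BP_BuildingFoundation at the preview transform, and holding rotate runs a looping timer that yaws it.
; Leaving build mode clears the preview's mesh without destroying the component and resets the DoOnce.
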(event Custom|Preview%20Tick
  (bind _camera (Variables|Default|GetCamera))
  (bind _returnvalue (Transformation|GetWorldLocation _camera))
  ;[0.4247 1 0.6963] Preview Tick
  (bind (_outhit _returnvalue_2) (Collision|LineTraceByChannel _returnvalue (+ _returnvalue (* (Math|Vector|GetForwardVector (Transformation|GetWorldRotation _camera)) 2e+03)) "TraceTypeQuery1" false 0 "None"))
  (if _returnvalue_2
    (Utilities|FlowControl|Sequence
      (:then_0
        (Utilities|FlowControl|DoOnce false
          (:Completed
            (bind _returnvalue_3 (Game|AddComponentbyClass (Variables|Default|GetPlayer%20Character) "/Script/Engine.StaticMeshComponent" false (Variables|Default|GetBuild%20Transform)))
            (bind _output_get (Variables|Default|SetPreview%20SM%20Component _returnvalue_3))
            (Components|StaticMesh|SetStaticMesh _output_get "/Game/BSTestLevel/Mesh/SM_Stylized_Wood_Foundation.SM_Stylized_Wood_Foundation")
            (Rendering|Material|SetMaterial _output_get 0 "/Game/BSTestLevel/Material/MAT_PreviewGreen.MAT_PreviewGreen")
            (Collision|SetCollisionEnabled _output_get "NoCollision"))))
      (:then_1
        (bind _output_get_2 (Variables|Default|SetBuild%20Transform (Math|Transform|MakeTransform (.Location (Collision|BreakHitResult _outhit)) (Variables|Default|GetBuild%20Transform%20Rotation) "1.000000,1.000000,1.000000")))
        (Transformation|SetWorldTransform (Variables|Default|GetPreview%20SM%20Component) _output_get_2 false false)))))

(event Custom|Reset%20Preview%20Tick%20Do%20Once
  ;[0.4247 1 0.6963] Preview Tick
  (Utilities|FlowControl|DoOnce false) ; enters at Reset
)

(event Custom|Rotate%20Preview
  ;[1 1 1] IA_RotateBuilding
  (Variables|Default|SetBuild%20Transform%20Rotation (Math|Rotator|CombineRotators (.rotation (Variables|Default|GetBuild%20Transform)) "0.000000,5.000000,0.000000")))

(event Input|EnhancedActionEvents|EnhancedInputActionIA_ToggleBuildMode
  (params (ActionValue :type Boolean) (ElapsedSeconds :type Float%20%28double-precision%29) (TriggeredSeconds :type Float%20%28double-precision%29) (InputAction :type Input%20Action%20Object%20Reference :default "/Game/BSTestLevel/Input/IA_ToggleBuildMode.IA_ToggleBuildMode"))
  ;[1 1 1] IA_ToggleBuildMode
  (:Started
    (Utilities|FlowControl|FlipFlop
      (:A
        (Variables|Default|SetIs%20Build%20Mode true))
      (:B
        (Variables|Default|SetIs%20Build%20Mode false)
        (Components|StaticMesh|SetStaticMesh (Variables|Default|GetPreview%20SM%20Component) 0)
        (CallFunction|ResetPreviewTickDoOnce)))))

(event Input|EnhancedActionEvents|EnhancedInputActionIA_PlaceBuilding
  (params (ActionValue :type Boolean) (ElapsedSeconds :type Float%20%28double-precision%29) (TriggeredSeconds :type Float%20%28double-precision%29) (InputAction :type Input%20Action%20Object%20Reference :default "/Game/BSTestLevel/Input/IA_PlaceBuilding.IA_PlaceBuilding"))
  ;[1 1 1] IA_PlaceBuilding
  (:Started
    (if (Variables|Default|GetIs%20Build%20Mode)
      (Game|SpawnActorfromClass "/Game/BSTestLevel/BP_BuildingFoundation.BP_BuildingFoundation_C" (Variables|Default|GetBuild%20Transform) "AlwaysSpawn" "MultiplyWithRoot" 0 0))))

(event Input|EnhancedActionEvents|EnhancedInputActionIA_RotateBuilding
  (params (ActionValue :type Boolean) (ElapsedSeconds :type Float%20%28double-precision%29) (TriggeredSeconds :type Float%20%28double-precision%29) (InputAction :type Input%20Action%20Object%20Reference :default "/Game/BSTestLevel/Input/IA_RotateBuilding.IA_RotateBuilding"))
  ;[1 1 1] IA_RotateBuilding
  (:Started
    (bind _returnvalue (Utilities|Time|SetTimerbyEvent (delegate Custom|Rotate%20Preview) 0.01 true)) ; 0.01초 마다 Rotate Preview 이벤트를 발생시킨다.
    (Variables|Default|SetRotateTimerHandle _returnvalue))
  (:Canceled
    (Utilities|Time|ClearandInvalidateTimerbyHandle (Variables|Default|GetRotateTimerHandle) :!label _label)
    (Variables|Default|SetRotateTimerHandle ""))
  (:Completed
    (goto _label)))

(event EventBeginPlay
  ;[1 1 1] BeginPlay
  (bind _asbp_bstest_character (Utilities|Casting|CastToBP_BSTestCharacter (Components|GetOwner)))
  (Variables|Default|SetPlayer%20Character _asbp_bstest_character)
  (Variables|Default|SetCamera (Variables|/Game/BSTestLevel/BP_BSTestCharacter.BP_BSTestCharacter_C|GetCamera _asbp_bstest_character)))

(event EventTick
  (params (DeltaSeconds :type Float%20%28single-precision%29))
  ;[1 1 1] Tick
  (if (Variables|Default|GetIs%20Build%20Mode)
    (CallFunction|PreviewTick)))