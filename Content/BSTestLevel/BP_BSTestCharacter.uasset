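; BP_BSTestCharacter is the player character Blueprint for the BSTest level, handling look, move and jump through Enhanced Input.
; On BeginPlay it adds the IMC_BSTestDefault mapping context to the local player subsystem of player controller 0.
; Look input drives controller yaw and pitch, and move input follows the full control rotation's right and forward vectors.
; Jump starts and stops with the jump action, while Tick, overlap and the construction script are empty.
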(event Input|EnhancedActionEvents|EnhancedInputActionIA_BSTestJump
  (params (ActionValue :type Boolean) (ElapsedSeconds :type Float%20%28double-precision%29) (TriggeredSeconds :type Float%20%28double-precision%29) (InputAction :type Input%20Action%20Object%20Reference :default "/Game/BSTestLevel/Input/IA_BSTestJump.IA_BSTestJump"))
  (:Started
    (Character|Jump))
  (:Completed
    (Character|StopJumping)))

(event Input|EnhancedActionEvents|EnhancedInputActionIA_BSTestMove
  (params (ActionValue :type Vector%202D%20Structure) (ElapsedSeconds :type Float%20%28double-precision%29) (TriggeredSeconds :type Float%20%28double-precision%29) (InputAction :type Input%20Action%20Object%20Reference :default "/Game/BSTestLevel/Input/IA_BSTestMove.IA_BSTestMove"))
  (bind (_x _y) (Math|Vector2D|BreakVector2D ActionValue))
  (bind _returnvalue (Pawn|GetControlRotation :!class /Script/Engine.Pawn))
  ;[1 1 1] Move
  (Pawn|Input|AddMovementInput (Math|Vector|GetRightVector _returnvalue) _x false)
  (Pawn|Input|AddMovementInput (Math|Vector|GetForwardVector _returnvalue) _y false))

(event Input|EnhancedActionEvents|EnhancedInputActionIA_BSTestLook
  (params (ActionValue :type Vector%202D%20Structure) (ElapsedSeconds :type Float%20%28double-precision%29) (TriggeredSeconds :type Float%20%28double-precision%29) (InputAction :type Input%20Action%20Object%20Reference :default "/Game/BSTestLevel/Input/IA_BSTestLook.IA_BSTestLook"))
  (bind (_x _y) (Math|Vector2D|BreakVector2D ActionValue))
  (bind _result (Math|Float|NegateFloat _x)
    (:%20%20
      (Pawn|Input|AddControllerYawInput _result)
      (Pawn|Input|AddControllerPitchInput _y))))

(event EventBeginPlay
  (Input|AddMappingContext (PlayerController|LocalPlayerSubsystems|GetEnhancedInputLocalPlayerSubsystem (Game|GetPlayerController 0)) "/Game/BSTestLevel/Input/IMC_BSTestDefault.IMC_BSTestDefault" 0 "(bIgnoreAllPressedKeysUntilRelease=True,bForceImmediately=False,bNotifyUserSettings=False)"))

(event Collision|EventActorBeginOverlap
  (params (OtherActor :type Actor%20Object%20Reference)))

(event EventTick
  (params (DeltaSeconds :type Float%20%28single-precision%29)))

(fn ConstructionScript)