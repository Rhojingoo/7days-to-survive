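; Projectile actor for the ranged zombie that damages the player on contact.
; When its collision component begins overlapping an actor other than its Spawner or itself, it calls Playerhit with fixed damage and SetHitSound if that actor is a C_GlobalPlayer, then destroys itself regardless of type.
; Casts to zombie and bullet classes trigger no action, and ignored overlaps only print the actor's name.
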(event OnComponentBeginOverlap(CollisionComponent)
  (params (OverlappedComponent :type Primitive%20Component%20Object%20Reference) (OtherActor :type Actor%20Object%20Reference) (OtherComp :type Primitive%20Component%20Object%20Reference) (OtherBodyIndex :type Integer) (bFromSweep :type Boolean) (SweepResult :type Hit%20Result%20Structure%20%28by%20ref%29))
  (Variables|Default|SetOther%20Actor OtherActor)
  (if (and (!= (Variables|Default|GetSpawner) (Variables|Default|GetOther%20Actor)) (!= (Variables|Default|GetOther%20Actor) self))
    (Utilities|FlowControl|Sequence
      (:then_0
        (bind _asc_global_player (Utilities|Casting|CastToC_GlobalPlayer (Variables|Default|GetOther%20Actor)))
        (Class|CGlobalPlayer|Playerhit _asc_global_player 10)
        (Class|CZombieBullet|SetHitSound))
      (:then_1
        (Utilities|Casting|CastToC_ZombieBase (Variables|Default|GetOther%20Actor)))
      (:then_2
        (Utilities|Casting|CastToC_ZombieBullet (Variables|Default|GetOther%20Actor)))
      (:then_3
        (Actor|DestroyActor)))
    (else
      (Development|PrintString (Utilities|GetDisplayName (Variables|Default|GetOther%20Actor))))))

(event EventBeginPlay)

(event Collision|EventActorBeginOverlap
  (params (OtherActor :type Actor%20Object%20Reference)))

(event EventTick
  (params (DeltaSeconds :type Float%20%28single-precision%29)))

(fn ConstructionScript)