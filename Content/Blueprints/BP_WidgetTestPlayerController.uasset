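; A test player controller that manages the in-game UI and a Tab-toggled menu for the inventory.
; On BeginPlay it creates the core in-game widget and adds it to the viewport.
; The Tab debug key flips a menu flag, creating a new UI manager widget above the core widget with the mouse cursor shown, or removing it and hiding the cursor.
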(event EventBeginPlay
  (bind _returnvalue (UserInterface|CreateWidget "/Game/Level/TestLevel/UI/WidgetBP/InGame/WB_InGameWidgetCore.WB_InGameWidgetCore_C"))
  (UserInterface|Viewport|AddtoViewport _returnvalue 0))

(event EventTick
  (params (DeltaSeconds :type Float%20%28single-precision%29)))

(event Input|KeyboardEvents|DebugKeyTab
  (params (Key :type Key%20Structure :default "None") (ActionValue :type Input%20Action%20Value%20Structure))
  ;[1 1 1] TAB키 -> 인벤토리 창 활성화
  (:Pressed
    (if (Variables|Default|GetIsMenuPopedUp)
      (Variables|Default|SetbShowMouseCursor false)
      (Widget|RemovefromParent (stale _returnvalue))
      (Variables|Default|SetIsMenuPopedUp false)
      (else
        (bind _returnvalue (UserInterface|CreateWidget "/Game/Level/TestLevel/UI/WidgetBP/InGame/WB_UIManager.WB_UIManager_C"))
        (Variables|Default|SetIsMenuPopedUp true)
        (Variables|Default|SetbShowMouseCursor true)
        (UserInterface|Viewport|AddtoViewport _returnvalue 1)))))

(fn ConstructionScript)